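; Target2 is a moving shootable target actor that destroys itself and the projectile when a BP_FirstPersonProjectile overlaps its sphere, printing a debug message.
; BeginPlay caches its transform and forward vector.
; Each Tick, MoveTarget applies a swept step built from that direction, SpawnSpeed and the starting rotation, without delta-time scaling.
; It also destroys itself once it strays Limit units from its start along world X.
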(event OnComponentBeginOverlap(Sphere1)
  (params (OverlappedComponent :type Primitive%20Component%20Object%20Reference) (OtherActor :type Actor%20Object%20Reference) (OtherComp :type Primitive%20Component%20Object%20Reference) (OtherBodyIndex :type Integer) (bFromSweep :type Boolean) (SweepResult :type Hit%20Result%20Structure%20%28by%20ref%29))
  (bind _asbp_first_person_projectile (Utilities|Casting|CastToBP_FirstPersonProjectile OtherActor))
  (Development|PrintString "Hello")
  (Actor|DestroyActor _asbp_first_person_projectile)
  (Actor|DestroyActor))

(event EventBeginPlay
  (bind _returnvalue (Transformation|GetActorTransform))
  (Variables|Default|SetRotation%20Factor _returnvalue)
  (Variables|Default|SetStartLocation _returnvalue)
  (Variables|Default|SetBallDirection (Transformation|GetActorForwardVector)))

(event EventTick
  (params (DeltaSeconds :type Float%20%28single-precision%29))
  (CallFunction|MoveTarget))

(fn ConstructionScript)

(fn MoveTarget
  (Transformation|SetActorTransform (Math|Conversions|ToTransform(Vector) (+ (Transformation|GetActorLocation) (* (+ (Variables|Default|GetBallDirection) (Variables|Default|GetSpawnSpeed)) (.rotation (Variables|Default|GetRotation%20Factor))))) true)
  (if (or (<= (.X (Math|Vector|BreakVector (Transformation|GetActorLocation))) (- (.X (Math|Vector|BreakVector (.location (Variables|Default|GetStartLocation)))) (Variables|Default|GetLimit))) (>= (.X (Math|Vector|BreakVector (Transformation|GetActorLocation))) (+ (.X (Math|Vector|BreakVector (.location (Variables|Default|GetStartLocation)))) (Variables|Default|GetLimit))))
    (Actor|DestroyActor)))