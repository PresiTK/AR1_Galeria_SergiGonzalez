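; Moving shooting target that awards points through GameManager when a first-person projectile overlaps its box, then destroys both projectile and target.
; Each Tick, MoveTarget makes a swept move using SpawnSpeed and the rotation captured at BeginPlay, without delta-time scaling.
; The target destroys itself once its X position reaches Limit distance either side of its start.
; DestroyTarget3 also exposes destruction as a separate function.
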(event OnComponentBeginOverlap(Box)
  (params (OverlappedComponent :type Primitive%20Component%20Object%20Reference) (OtherActor :type Actor%20Object%20Reference) (OtherComp :type Primitive%20Component%20Object%20Reference) (OtherBodyIndex :type Integer) (bFromSweep :type Boolean) (SweepResult :type Hit%20Result%20Structure%20%28by%20ref%29))
  ;[1 1 1] Detecta si el Projectill overlapea en el objeto y si sucede destruye el projectil , el objeto y llama a la Funcion Target3AddPoints
  (bind _asbp_first_person_projectile (Utilities|Casting|CastToBP_FirstPersonProjectile OtherActor))
  (bind _outactors (Actor|GetAllActorsOfClass "/Game/CORREGIR/Blueprints/GameManager.GameManager_C"))
  (Default|Target3AddPoints _outactors)
  (Actor|DestroyActor _asbp_first_person_projectile)
  (Actor|DestroyActor))

(event EventBeginPlay
  (bind _returnvalue (Transformation|GetActorTransform))
  ;[1 1 1] Setea RotationFactor y Start location, y ball direction(se puede modificar quitando esteo)
  (Variables|Default|SetRotation%20Factor _returnvalue)
  (Variables|Default|SetStartLocation _returnvalue)
  (Variables|Default|SetBallDirection (Transformation|GetActorForwardVector)))

(event EventTick
  (params (DeltaSeconds :type Float%20%28single-precision%29))
  ;[1 1 1] Lla a la Función move Target en cada Tick
  (CallFunction|MoveTarget))

(fn ConstructionScript)

(fn MoveTarget
  ;[1 1 1] Funcion que hace que se muevan los Target a la Velocidad modificable en SpawnSpeed como un vector y que si recorre 2000 destruye al actor
  (Transformation|SetActorTransform (Math|Conversions|ToTransform(Vector) (+ (Transformation|GetActorLocation) (* (Variables|Default|GetSpawnSpeed) (.rotation (Variables|Default|GetRotation%20Factor))))) true)
  (if (or (<= (.X (Math|Vector|BreakVector (Transformation|GetActorLocation))) (- (.X (Math|Vector|BreakVector (.location (Variables|Default|GetStartLocation)))) (Variables|Default|GetLimit))) (>= (.X (Math|Vector|BreakVector (Transformation|GetActorLocation))) (+ (.X (Math|Vector|BreakVector (.location (Variables|Default|GetStartLocation)))) (Variables|Default|GetLimit))))
    (Actor|DestroyActor)))

(fn DestroyTarget3
  ;[1 1 1] Funcion que Destruye Target3
  (Actor|DestroyActor))