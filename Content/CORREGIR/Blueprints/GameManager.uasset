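; GameManager Blueprint that runs a countdown once something has been picked up, ending with a "START!" message.
; Obtained sets the HasBeenPicked flag, which Tick checks while Timer is non-negative.
; A Delay inside Tick paces TimerFunction to roughly one call per second.
; TimerFunction prints and decrements Timer, showing output only through PrintString, and announces the start when it drops below zero.
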(event EventTick
  (params (DeltaSeconds :type Float%20%28single-precision%29))
  (if (<= 0.0 (Variables|Default|GetTimer))
    (if (Variables|Default|GetHasBeenPicked)
      (Utilities|FlowControl|Delay 1.0)
      (CallFunction|TimerFunction))
    (elif (<= 0.0 (Variables|Default|GetTimer))
      _)))

(fn ConstructionScript)

(fn Obtained
  (Variables|Default|SetHasBeenPicked true))

(fn TimerFunction
  (Development|PrintString (Utilities|String|ToString(Float) (Variables|Default|GetTimer)))
  (Variables|Default|SetTimer (- (Variables|Default|GetTimer) 1.0))
  (if (< (Variables|Default|GetTimer) 0.0)
    (Development|PrintString "START!")))