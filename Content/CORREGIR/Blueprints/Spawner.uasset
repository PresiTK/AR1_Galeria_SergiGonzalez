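; Spawner actor that spawns target actors at its BeginPlay transform while enabled, with GameCondition and GameEnd switching spawning on and off.
; Tick runs through a Delay of SpawnTime before calling Spawn, using the latent node as a repeating timer.
; Spawn selects one of three target classes from the ChangeTarget countdown, which resets to RestartChange after reaching zero, cycling the types.
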(event EventBeginPlay
  (Variables|Default|SetSpawnPosition (Transformation|GetActorTransform)))

(event EventTick
  (params (DeltaSeconds :type Float%20%28single-precision%29))
  (if (Variables|Default|GetStartSpawn)
    (Utilities|FlowControl|Delay (Variables|Default|GetSpawnTime))
    (CallFunction|Spawn)))

(fn ConstructionScript)

(fn Spawn
  (switch int (Variables|Default|GetChangeTarget)
    (:0
      (Game|SpawnActorfromClass "/Game/CORREGIR/Blueprints/Target1.Target1_C" (Variables|Default|GetSpawnPosition) "AlwaysSpawn" "MultiplyWithRoot" 0 0)
      (Variables|Default|SetChangeTarget (Variables|Default|GetRestartChange)))
    (:1
      (Game|SpawnActorfromClass "/Game/CORREGIR/Blueprints/Target3.Target3_C" (Variables|Default|GetSpawnPosition) "AlwaysSpawn" "MultiplyWithRoot" 0 0)
      (Variables|Default|SetChangeTarget (- (Variables|Default|GetChangeTarget) 1)))
    (:2
      (Game|SpawnActorfromClass "/Game/CORREGIR/Blueprints/Target2.Target2_C" (Variables|Default|GetSpawnPosition) "AlwaysSpawn" "MultiplyWithRoot" 0 0)
      (Variables|Default|SetChangeTarget (- (Variables|Default|GetChangeTarget) 1)))))

(fn GameCondition
  (Variables|Default|SetStartSpawn true))

(fn GameEnd
  (Variables|Default|SetStartSpawn false))